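; RTS camera with a spring arm that pans by screen-edge mouse scrolling or WASD and zooms on input.
; IsScrolling checks the cursor against thin viewport edge margins, moves the actor with swept local offsets and returns the scroll side.
; MouseScrolling and WSADScrolling flags keep the two pan methods from overlapping.
; Zoom inputs set a clamped target length that Tick eases the spring arm toward.
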(event `InputAxis|MouseAxis`
  (params (AxisValue :type "Float (single-precision)"))
  ;[1 1 1] Camera move by mouse
  (if (not (`self.WSADScrolling`))
    (set `self.MouseScrolling` true)
    (`self.IsScrolling`)))

(event `self.ReceiveBeginPlay`
  (bind _returnvalue (`GameplayStatics.GetPlayerController` 0))
  (bind (_sizex _sizey) (`PlayerController.GetViewportSize` _returnvalue))
  ;[1 1 1] Begin Play
  (`self.SetDefaultCamSettings`)
  (set `PlayerController.bShowMouseCursor` true _returnvalue)
  (`PlayerController.SetMouseLocation` _returnvalue (/ _sizex 2) (/ _sizey 2)))

(event `SetDefaultCamSettings`
  ;[1 1 1] Set Default Camera Settings
  (bind _output_get (set `self.CurrentCamZoom` (`self.CurrentCamZoom`)))
  (set `SpringArmComponent.TargetArmLength` _output_get (`self.SpringArm`)))

(event `self.ReceiveTick`
  (params (DeltaSeconds :type "Float (single-precision)"))
  (bind _springarm (`self.SpringArm`))
  ;[1 1 1] Update camera zoom
  (set `SpringArmComponent.TargetArmLength` (`KismetMathLibrary.FInterpTo` (`SpringArmComponent.TargetArmLength` _springarm) (`self.DesireCamZoom`) DeltaSeconds 5.0) _springarm))

(event `InputAction|ZoomIn`
  (params (Key :type "Key Structure"))
  ;[1 1 1] Camera Zoom
  (:`Pressed`
    (set `self.DesireCamZoom` (`KismetMathLibrary.FClamp` (+ (`self.DesireCamZoom`) (* (`self.CamZoomSpeed`) -1.0)) (`self.MinCamZoom`) (`self.MaxCamZoom`)))))

(event `InputAction|ZoomOut`
  (params (Key :type "Key Structure"))
  ;[1 1 1] Camera Zoom
  (:`Pressed`
    (set `self.DesireCamZoom` (`KismetMathLibrary.FClamp` (+ (`self.DesireCamZoom`) (`self.CamZoomSpeed`)) (`self.MinCamZoom`) (`self.MaxCamZoom`)))))

(event `InputAxis|MoveForward`
  (params (AxisValue :type "Float (single-precision)"))
  ;[1 1 1] Camera move by WASD
  (if (not (`self.MouseScrolling`))
    (set `self.WSADScrolling` true)
    (`self.K2_AddActorLocalOffset` (`KismetMathLibrary.MakeVector` (* AxisValue (`self.CamMoveSpeed`))) true)
    (set `self.WSADScrolling` false)))

(event `InputAxis|MoveRight`
  (params (AxisValue :type "Float (single-precision)"))
  ;[1 1 1] Camera move by WASD
  (if (not (`self.MouseScrolling`))
    (set `self.WSADScrolling` true)
    (`self.K2_AddActorLocalOffset` (`KismetMathLibrary.MakeVector` 0.0 (* AxisValue (`self.CamMoveSpeed`))) true)
    (set `self.WSADScrolling` false)))

(fn `Get Scroll Direction`
  (returns (Direction :type "Vector Structure"))
  (bind (_locationx _locationy) (`PlayerController.GetMousePosition` (`GameplayStatics.GetPlayerController` 0)))
  (return (`KismetMathLibrary.MakeVector` (.y (`KismetMathLibrary.ClampVectorSize` (* (`KismetMathLibrary.Conv_Vector2DToVector` (- (`KismetMathLibrary.MakeVector2D` _locationx _locationy) (/ (`WidgetLayoutLibrary.GetViewportSize`) 2.0))) -1.0) 0.2 1.0)) (* (.x (`KismetMathLibrary.ClampVectorSize` (* (`KismetMathLibrary.Conv_Vector2DToVector` (- (`KismetMathLibrary.MakeVector2D` _locationx _locationy) (/ (`WidgetLayoutLibrary.GetViewportSize`) 2.0))) -1.0) 0.2 1.0)) -1.0))))

(fn `IsScrolling`
  (returns (ScrollSide :type "/Game/Blueprints/Character/ECameraScroll Enum"))
  (bind (_x _y) (`KismetMathLibrary.BreakVector2D` (`WidgetLayoutLibrary.GetViewportSize`)))
  (bind (_x_2 _y_2) (`KismetMathLibrary.BreakVector2D` (`WidgetLayoutLibrary.GetViewportSize`)))
  (bind (_locationx _locationy) (`PlayerController.GetMousePosition` (`GameplayStatics.GetPlayerController` 0)))
  (bind (_locationx_2 _locationy_2) (`PlayerController.GetMousePosition` (`GameplayStatics.GetPlayerController` 0)))
  (bind _returnvalue (< _locationx (* _x_2 0.03)))
  (bind _returnvalue_2 (< _locationy (* _y_2 0.03)))
  (bind _returnvalue_3 (and (not _returnvalue) (> _locationx_2 (* _x 0.97))))
  (bind _returnvalue_4 (and (not _returnvalue_2) (> _locationy_2 (* _y 0.97))))
  ;[1 1 1] Calculate scroll side
  (`|ExecutionSequence`
    (:`then_0`
      ;[1 1 1] Moving camera
      (if _returnvalue
        (set `self.ScrollSide` "NewEnumerator2")
        (`self.K2_AddActorLocalOffset` (`KismetMathLibrary.MakeVector` 0.0 (* (`self.CamMoveSpeed`) -1.0)) true)))
    (:`then_1`
      (if _returnvalue_3
        (set `self.ScrollSide` "NewEnumerator1")
        (`self.K2_AddActorLocalOffset` (`KismetMathLibrary.MakeVector` 0.0 (`self.CamMoveSpeed`)) true)))
    (:`then_2`
      (if _returnvalue_2
        (set `self.ScrollSide` "NewEnumerator3")
        (`self.K2_AddActorLocalOffset` (`KismetMathLibrary.MakeVector` (`self.CamMoveSpeed`)) true)))
    (:`then_3`
      (if _returnvalue_4
        (set `self.ScrollSide` "NewEnumerator4")
        (`self.K2_AddActorLocalOffset` (`KismetMathLibrary.MakeVector` (* (`self.CamMoveSpeed`) -1.0)) true)))
    (:`then_4`
      ;[1 1 1] Calculate if no scroll
      (if (not (or _returnvalue _returnvalue_3 _returnvalue_2 _returnvalue_4))
        (set `self.MouseScrolling` false)
        (set `self.ScrollSide` "NewEnumerator0")))
    (:`then_5`
      (return (`self.ScrollSide`)))))

(fn `UserConstructionScript`)