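; ClickerController is a gameplay Blueprint that records mouse input into the game's shared GameInfoInstance.
; On BeginPlay it casts and caches the game instance.
; Left click input actions increment TotalClicks and set or clear LMBPressed, while right click actions only set or clear RMBPressed.
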(event `self.ReceiveBeginPlay`
  (bind _asgame_info_instance (cast `/Game/Blueprints/AllLevels/GameInfoInstance` (`GameplayStatics.GetGameInstance`)))
  (set `self.GameInstanceRef` _asgame_info_instance))

(event `InputAction|Left Mouse Click`
  (params (Key :type "Key Structure"))
  (bind _gameinstanceref (`self.GameInstanceRef`))
  (:`Pressed`
    (set `/Game/Blueprints/AllLevels/GameInfoInstance.TotalClicks` (+ (`/Game/Blueprints/AllLevels/GameInfoInstance.TotalClicks` _gameinstanceref) 1) _gameinstanceref)
    (set `/Game/Blueprints/AllLevels/GameInfoInstance.LMBPressed?` true (`self.GameInstanceRef`)))
  (:`Released`
    (set `/Game/Blueprints/AllLevels/GameInfoInstance.LMBPressed?` false (`self.GameInstanceRef`))))

(event `InputAction|Right Mouse Click`
  (params (Key :type "Key Structure"))
  (bind _gameinstanceref (`self.GameInstanceRef`))
  (:`Pressed`
    (set `/Game/Blueprints/AllLevels/GameInfoInstance.RMBPressed?` true _gameinstanceref))
  (:`Released`
    (set `/Game/Blueprints/AllLevels/GameInfoInstance.RMBPressed?` false _gameinstanceref)))

(fn `UserConstructionScript`)