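; RTS camera that pans and zooms over the world with a visible mouse cursor.
; WASD axes move the actor by swept local offsets, and the zoom axis adjusts the clamped spring arm length.
; The MouseAxis event runs IsScrolling, which pans when the cursor nears a viewport edge and records the side in an enum.
; GetScrollDirection derives a direction from the cursor's offset to screen center but is not called in these graphs.
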(event `InputAxis|MouseAxis`
  (params (AxisValue :type "Float (single-precision)"))
  (`self.IsScrolling`))

(event `self.ReceiveBeginPlay`
  (`self.SetDefaultCamSettings`)
  (set `PlayerController.bShowMouseCursor` true (`GameplayStatics.GetPlayerController` 0)))

(event `SetDefaultCamSettings`
  ;[1 1 1] Set Default Camera Settings
  (bind _output_get (set `self.CurrentCamZoom` (`self.CurrentCamZoom`)))
  (set `SpringArmComponent.TargetArmLength` _output_get (`self.SpringArm`)))

(event `InputAxis|CamZoom`
  (params (AxisValue :type "Float (single-precision)"))
  (bind _springarm (`self.SpringArm`))
  ;[1 1 1] Camera Zoom
  (set `SpringArmComponent.TargetArmLength` (`KismetMathLibrary.FClamp` (+ (* AxisValue (`self.CapZoomSpeed`) -1.0) (`SpringArmComponent.TargetArmLength` _springarm)) (`self.MinCamZoom`) (`self.MaxCamZoom`)) _springarm))

(event `InputAxis|MoveForward`
  (params (AxisValue :type "Float (single-precision)"))
  ;[1 1 1] Camera move by WASD
  (`self.K2_AddActorLocalOffset` (`KismetMathLibrary.MakeVector` (* AxisValue (`self.CamMoveSpeed`))) true))

(event `InputAxis|MoveRight`
  (params (AxisValue :type "Float (single-precision)"))
  ;[1 1 1] Camera move by WASD
  (`self.K2_AddActorLocalOffset` (`KismetMathLibrary.MakeVector` 0.0 (* AxisValue (`self.CamMoveSpeed`))) true))

(fn `Get Scroll Direction`
  (returns (Direction :type "Vector Structure"))
  (bind (_locationx _locationy) (`PlayerController.GetMousePosition` (`GameplayStatics.GetPlayerController` 0)))
  (return (`KismetMathLibrary.MakeVector` (.y (`KismetMathLibrary.ClampVectorSize` (* (`KismetMathLibrary.Conv_Vector2DToVector` (- (`KismetMathLibrary.MakeVector2D` _locationx _locationy) (/ (`WidgetLayoutLibrary.GetViewportSize`) 2.0))) -1.0) 0.2 1.0)) (* (.x (`KismetMathLibrary.ClampVectorSize` (* (`KismetMathLibrary.Conv_Vector2DToVector` (- (`KismetMathLibrary.MakeVector2D` _locationx _locationy) (/ (`WidgetLayoutLibrary.GetViewportSize`) 2.0))) -1.0) 0.2 1.0)) -1.0))))

(fn `IsScrolling`
  (returns (ScrollSide :type "/Game/Blueprints/Characters/ECameraScroll Enum"))
  (bind (_x _y) (`KismetMathLibrary.BreakVector2D` (`WidgetLayoutLibrary.GetViewportSize`)))
  (bind (_locationx _locationy) (`PlayerController.GetMousePosition` (`GameplayStatics.GetPlayerController` 0)))
  (bind (_x_2 _y_2) (`KismetMathLibrary.BreakVector2D` (`WidgetLayoutLibrary.GetViewportSize`)))
  (bind (_locationx_2 _locationy_2) (`PlayerController.GetMousePosition` (`GameplayStatics.GetPlayerController` 0)))
  (bind (_locationx_3 _locationy_3) (`PlayerController.GetMousePosition` (`GameplayStatics.GetPlayerController` 0)))
  (bind _returnvalue (< _locationx_2 (* _x_2 0.03)))
  (bind _returnvalue_2 (< _locationy_2 (* _y_2 0.03)))
  (`|ExecutionSequence`
    (:`then_0`
      (if _returnvalue
        (set `self.ScrollSide` "NewEnumerator2")
        (`self.K2_AddActorLocalOffset` (`KismetMathLibrary.MakeVector` 0.0 (* (`self.CamMoveSpeed`) -1.0)) true)))
    (:`then_1`
      (if (and (not _returnvalue) (> _locationx_3 (* _x 0.97)))
        (set `self.ScrollSide` "NewEnumerator1")
        (`self.K2_AddActorLocalOffset` (`KismetMathLibrary.MakeVector` 0.0 (`self.CamMoveSpeed`)) true)))
    (:`then_2`
      (if _returnvalue_2
        (set `self.ScrollSide` "NewEnumerator3")
        (`self.K2_AddActorLocalOffset` (`KismetMathLibrary.MakeVector` (`self.CamMoveSpeed`)) true)))
    (:`then_3`
      (if (and (not _returnvalue_2) (> _locationy_3 (* _y 0.97)))
        (set `self.ScrollSide` "NewEnumerator4")
        (`self.K2_AddActorLocalOffset` (`KismetMathLibrary.MakeVector` (* (`self.CamMoveSpeed`) -1.0)) true)))
    (:`then_4`
      (if (and (== _locationx 0.0) (== _locationy 0.0))
        (set `self.ScrollSide` "NewEnumerator0")))
    (:`then_5`
      (return (`self.ScrollSide`)))))

(fn `UserConstructionScript`)