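; PacanActor is a clickable tutorial guide that teaches camera movement, inventory, crafting and combat through a DialogWB widget tracking its screen position.
; Each sphere click passes a DoOnce gate into a counter-driven step that sets the dialog text.
; Delay loops poll GameInstance usage flags or spawned Tutorial_Creep health before re-arming the gate.
; The four-creep wave check ANDs their health, so one death is enough to advance.
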(event `self.ReceiveBeginPlay`
  (bind _returnvalue (`|CreateWidget` "/Game/UI/GamePlay/DialogWB.DialogWB_C" (`GameplayStatics.GetPlayerController` 0)))
  (bind _output_get (set `self.DialogRef` _returnvalue))
  (`Widget.SetVisibility` _output_get "Visible")
  (`UserWidget.AddToViewport` _output_get 0)
  (bind _asgame_info_instance (cast `/Game/Blueprints/AllLevels/GameInfoInstance` (`GameplayStatics.GetGameInstance`)))
  (set `self.GameInstanceRef` _asgame_info_instance))

(event `self.ReceiveTick`
  (params (DeltaSeconds :type "Float (single-precision)"))
  (`UserWidget.SetPositionInViewport` (`self.DialogRef`) (+ (`GameplayStatics.ProjectWorldToScreen` (`GameplayStatics.GetPlayerController` 0) (`self.K2_GetActorLocation` self)) (75.0 -75.0)) true)
  (`TextBlock.SetText` (`/Game/UI/GamePlay/DialogWB.DialogText` (`self.DialogRef`)) (`self.DialogString`)))

(event `self.Sphere.OnClicked`
  (params (TouchedComponent :type "PrimitiveComponent Object Reference") (ButtonPressed :type "Key Structure"))
  (`/Engine/EditorBlueprintResources/StandardMacros.DoOnce` false :!label _label
    (:`Completed`
      (bind _result (`/Engine/EditorBlueprintResources/StandardMacros.IncrementInt` (`self.WhichEntrance`))
        (:`  `
          (switch `int` _result
            (:`0`
              (set `self.DialogString` "Camera movement can be changed in settings. You can move camera with WASD or mouse. Not recommended to switch off both of them. Click me to next advice")
              (`KismetSystemLibrary.Delay` 1.0)
              (`self.ResetDoOnce`))
            (:`1`
              (set `self.DialogString` "Exellent!")
              (`KismetSystemLibrary.Delay` 0.6)
              (set `self.DialogString` "Now open Inventory - press I then click me")
              (`KismetSystemLibrary.Delay` 1.0 :!label _label_2)
              (if (`/Game/Blueprints/AllLevels/GameInfoInstance.InventoryUsed?` (`self.GameInstanceRef`))
                (`self.ResetDoOnce`)
                (else
                  (goto _label_2))))
            (:`2`
              (set `self.DialogString` "Also you can open craft - press C then click me")
              (`KismetSystemLibrary.Delay` 1.0 :!label _label_3)
              (if (`/Game/Blueprints/AllLevels/GameInfoInstance.CraftUsed?` (`self.GameInstanceRef`))
                (`self.ResetDoOnce`)
                (else
                  (goto _label_3))))
            (:`3`
              (set `self.DialogString` "Krasavello!")
              (`KismetSystemLibrary.Delay` 0.6)
              (bind _returnvalue (`|SpawnActorFromClass` "/Game/Blueprints/AI/Creeps/Tutorial_Creep.Tutorial_Creep_C" (`KismetMathLibrary.Conv_VectorToTransform` (+ (`SceneComponent.K2_GetComponentLocation` (`self.Sphere`)) (-500.0 -1000.0 0.0))) "Undefined" "OverrideRootScale" null 150.0 150.0 0 0 0 "Simple Creep" null))
              (set `self.DialogString` "There is a creep, it's your enemy! Let's craft a knife and kill this guy")
              (`KismetSystemLibrary.Delay` 10.0)
              (set `self.DialogString` "There is a creep, it's your enemy! Let's craft a knife and kill this guy, also you need to equip weapon with RMB on them and click \"Use\"")
              (`KismetSystemLibrary.Delay` 0.1 :!label _label_4)
              (if (> (`/Game/Blueprints/AI/Creeps/Creep_Character.CurrentHealth` _returnvalue) 0.0)
                (goto _label_4)
                (else
                  (set `self.DialogString` "Good job! Now kill 4 more then click me")
                  (`KismetSystemLibrary.Delay` 1.0)
                  (bind _returnvalue_2 (`|SpawnActorFromClass` "/Game/Blueprints/AI/Creeps/Tutorial_Creep.Tutorial_Creep_C" (`KismetMathLibrary.Conv_VectorToTransform` (+ (`SceneComponent.K2_GetComponentLocation` (`self.Sphere`)) (-500.0 -1000.0 0.0))) "Undefined" "OverrideRootScale" null 150.0 150.0 0 0 0 "Simple Creep" null))
                  (`KismetSystemLibrary.Delay` 1.0)
                  (bind _returnvalue_3 (`|SpawnActorFromClass` "/Game/Blueprints/AI/Creeps/Tutorial_Creep.Tutorial_Creep_C" (`KismetMathLibrary.Conv_VectorToTransform` (+ (`SceneComponent.K2_GetComponentLocation` (`self.Sphere`)) (-500.0 -800.0 0.0))) "Undefined" "OverrideRootScale" null 150.0 150.0 0 0 0 "Simple Creep" null))
                  (`KismetSystemLibrary.Delay` 1.0)
                  (bind _returnvalue_4 (`|SpawnActorFromClass` "/Game/Blueprints/AI/Creeps/Tutorial_Creep.Tutorial_Creep_C" (`KismetMathLibrary.Conv_VectorToTransform` (+ (`SceneComponent.K2_GetComponentLocation` (`self.Sphere`)) (-500.0 -600.0 0.0))) "Undefined" "OverrideRootScale" null 150.0 150.0 0 0 0 "Simple Creep" null))
                  (`KismetSystemLibrary.Delay` 1.0)
                  (bind _returnvalue_5 (`|SpawnActorFromClass` "/Game/Blueprints/AI/Creeps/Tutorial_Creep.Tutorial_Creep_C" (`KismetMathLibrary.Conv_VectorToTransform` (+ (`SceneComponent.K2_GetComponentLocation` (`self.Sphere`)) (-500.0 -400.0 0.0))) "Undefined" "OverrideRootScale" null 150.0 150.0 0 0 0 "Simple Creep" null))
                  (`KismetSystemLibrary.Delay` 0.1 :!label _label_5)
                  (if (and (> (`/Game/Blueprints/AI/Creeps/Creep_Character.CurrentHealth` _returnvalue_2) 0.0) (> (`/Game/Blueprints/AI/Creeps/Creep_Character.CurrentHealth` _returnvalue_3) 0.0) (> (`/Game/Blueprints/AI/Creeps/Creep_Character.CurrentHealth` _returnvalue_4) 0.0) (> (`/Game/Blueprints/AI/Creeps/Creep_Character.CurrentHealth` _returnvalue_5) 0.0))
                    (goto _label_5)
                    (else
                      (`self.ResetDoOnce`))))))
            (:`4`
              (set `self.DialogString` "Nice! Also you can make new weapon -> pick up steel which droped under creeps and craft Blade then Grip and put them together!!"))))))))

(event `ResetDoOnce`
  (goto _label :!via `Reset`))

(fn `UserConstructionScript`)