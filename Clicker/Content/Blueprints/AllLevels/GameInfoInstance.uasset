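; Game instance that handles menu navigation, player progress and saving across levels.
; Show events open the main menu and loading screen levels, or display Settings and LevelSelect widgets, creating them when missing.
; EndLevel sets next-level availability, records stats, gold and cursor info in the player info struct, saves it, then shows the stats widget.
; LoadGame only stores the loaded slot reference, and PutOnWeapon is an empty stub.
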(event `ShowMainMenu`
  ;[1 1 1] Show Main Menu and Enable Mouse Control
  (`GameplayStatics.OpenLevel` "MainMenu"))

(event `ShowSettings`
  (bind _returnvalue (`GameplayStatics.GetPlayerController` 0))
  ;[1 1 1] Show Settings and Enable Mouse Control
  (`/Engine/EditorBlueprintResources/StandardMacros.IsValid` (`self.Settings_WB`)
    (:`Is Valid`
      _)
    (:`Is Not Valid`
      (bind _returnvalue_2 (`|CreateWidget` "/Game/UI/MainMenu/Settings.Settings_C" _returnvalue))
      (set `self.Settings_WB` _returnvalue_2)))
  (`UserWidget.AddToViewport` (`self.Settings_WB`) 0)
  (set `PlayerController.bShowMouseCursor` true _returnvalue))

(event `ShowLevelSelect`
  (bind _returnvalue (`GameplayStatics.GetPlayerController` 0))
  ;[1 1 1] Show select level and Enable Mouse Control
  (`/Engine/EditorBlueprintResources/StandardMacros.IsValid` (`self.LevelSelect_WB`)
    (:`Is Valid`
      _)
    (:`Is Not Valid`
      (bind _returnvalue_2 (`|CreateWidget` "/Game/UI/MainMenu/LevelSelect.LevelSelect_C" _returnvalue))
      (set `self.LevelSelect_WB` _returnvalue_2)))
  (`UserWidget.AddToViewport` (`self.LevelSelect_WB`) 0)
  (set `PlayerController.bShowMouseCursor` true _returnvalue))

(event `SaveGame`
  (bind _savegame_ref (`self.SaveGame_Ref`))
  ;[1 1 1] Save game event
  (`/Engine/EditorBlueprintResources/StandardMacros.IsValid` (`self.SaveGame_Ref`)
    (:`Is Valid`
      _)
    (:`Is Not Valid`
      (bind _returnvalue (`GameplayStatics.CreateSaveGameObject` "/Game/Blueprints/AllLevels/PlayerSaveGame.PlayerSaveGame_C"))
      (bind _asplayer_save_game (cast `/Game/Blueprints/AllLevels/PlayerSaveGame` _returnvalue))
      (set `self.SaveGame_Ref` _asplayer_save_game)))
  (set `/Game/Blueprints/AllLevels/PlayerSaveGame.S_PlayerInfo` (`self.S_PlayerInfo`) _savegame_ref)
  (`GameplayStatics.SaveGameToSlot` _savegame_ref (`self.PlayerInfoSave`)))

(event `LoadGame`
  ;[1 1 1] Load Game
  (bind _returnvalue (`GameplayStatics.LoadGameFromSlot` (`self.PlayerInfoSave`)))
  (set `self.LoadedGame_Ref` _returnvalue))

(event `ShowLoadingScreen`
  ;[1 1 1] Show loadnig Screen
  (`GameplayStatics.OpenLevel` "LoadingScreen"))

(event `EditCursorSettings`
  (params (UpdatedCursorInfo :type "/Game/Blueprints/Items/WeaponInfo Structure"))
  ;[1 1 1] Saving cursor settings
  (set `self.CursorInfo` UpdatedCursorInfo))

(event `EndLevel`
  (params (`IsDone?` :type Boolean))
  (bind _levelid (`self.LevelID`))
  (bind (_availablelevel _levelstats) (break `/Game/Blueprints/AllLevels/PlayerInfo` (`self.S_PlayerInfo`)))
  (bind _levelstats_2 (make `/Game/Blueprints/AllLevels/LevelStats` _levelid (`self.TimePlayed`) (`self.Score`) (`self.MaxEnemies`) (`self.KilledEnemy`) (`self.ClicksOnCreeps`) (`self.LevelName`) `IsDone?` (`self.TotalClicks`)))
  ;[1 1 1] Creating EndGameStats
  ;;[1 1 1] Setting Level Progress
  (`KismetArrayLibrary.Array_Set` _availablelevel (+ (`self.LevelID`) 1) `IsDone?`)
  ;;[1 1 1] Setting LevelStats
  (`KismetArrayLibrary.Array_Set` _levelstats _levelid _levelstats_2)
  ;;[1 1 1] Setting gold and cursor info
  (set `self.S_PlayerInfo` (make `/Game/Blueprints/AllLevels/PlayerInfo` _availablelevel _levelstats (`self.Gold`) (`self.CursorInfo`)))
  ;;[1 1 1] Saving Information
  (`self.SaveGame`)
  ;;[1 1 1] Drawing EndGameStats with variables
  (bind _returnvalue (`|CreateWidget` "/Game/UI/GamePlay/EndLevelStats.EndLevelStats_C" null _levelstats_2))
  (`UserWidget.AddToViewport` _returnvalue 0))

(event `PutOnWeapon`
  (params (`Weapon to wear` :type "/Game/Blueprints/Items/S_ItemInfo Structure")))