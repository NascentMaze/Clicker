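; IsFinish is a behavior tree decorator condition that tests an AI's progress along a set of route points.
; PerformConditionCheck gathers all RoutePoints actors in the level and compares their count to the CheckpointNum Blackboard integer.
; Despite its name, it passes while the two numbers differ and fails once they are equal.
; The EventGraph holds only an unconnected copy of the same logic.
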(fn `PerformConditionCheck`
  (params (OwnerActor :type "Actor Object Reference"))
  (returns (ReturnValue :type Boolean))
  (bind _outactors (`GameplayStatics.GetAllActorsOfClass` "/Game/Blueprints/AI/RoutePoints.RoutePoints_C"))
  (return (!= (`KismetArrayLibrary.Array_Length` _outactors) (`BTFunctionLibrary.GetBlackboardValueAsInt` (`self.CheckpointNum`)))))