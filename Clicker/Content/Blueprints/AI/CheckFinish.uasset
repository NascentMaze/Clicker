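; Behavior tree task that checks whether an AI has reached the end of its route and destroys it if so.
; It compares the number of RoutePoints actors in the level with the CheckpointNum blackboard value, and on a match destroys the SelfActor.
; Both branches print debug strings and finish with success, so the task never fails the tree.
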(event `self.ReceiveExecute`
  (params (OwnerActor :type "Actor Object Reference"))
  (bind _outactors (`GameplayStatics.GetAllActorsOfClass` "/Game/Blueprints/AI/RoutePoints.RoutePoints_C"))
  (if (== (`KismetArrayLibrary.Array_Length` _outactors) (`BTFunctionLibrary.GetBlackboardValueAsInt` (`self.CheckpointNum`)))
    (`KismetSystemLibrary.PrintString` "True")
    (`Actor.K2_DestroyActor` (`BTFunctionLibrary.GetBlackboardValueAsActor` (`self.SelfActor`)))
    (`KismetSystemLibrary.PrintString` "Destroyed")
    (`self.FinishExecute` true)
    (else
      (`KismetSystemLibrary.PrintString` "False")
      (`self.FinishExecute` true))))