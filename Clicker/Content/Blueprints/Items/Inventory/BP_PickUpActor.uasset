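; BP_PickUpActor is a clickable world item that adds itself to the player's inventory.
; BeginPlay enables click events on the player controller, and clicking the static mesh passes its item class and amount to the InventoryRef of the controlled Clicker_Character.
; A successful add keeps any remainder as the new amount, or destroys the actor when nothing is left.
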(event `self.ReceiveBeginPlay`
  (set `PlayerController.bEnableClickEvents` true (`GameplayStatics.GetPlayerController` 0)))

(event `self.StaticMesh.OnClicked`
  (params (TouchedComponent :type "PrimitiveComponent Object Reference") (ButtonPressed :type "Key Structure"))
  (`KismetSystemLibrary.PrintString` "Click recieved")
  (bind _asclicker_character (cast `/Game/Blueprints/Character/Clicker_Character` (`Controller.K2_GetPawn` (`GameplayStatics.GetPlayerController` 0))))
  (bind _inventory_ref (`/Game/Blueprints/Character/Clicker_Character.Inventory_Ref` _asclicker_character))
  (`/Engine/EditorBlueprintResources/StandardMacros.IsValid` _inventory_ref
    (:`Is Valid`
      (bind (_succes_ _rest) (`/Game/Blueprints/Items/Inventory/BP_Inventory.AddItem` _inventory_ref (`self.ItemToAdd`) (`self.Amount`)))
      (if _succes_
        (if (> _rest 0)
          (set `self.Amount` _rest)
          (else
            (`self.K2_DestroyActor`)))))))

(fn `UserConstructionScript`)