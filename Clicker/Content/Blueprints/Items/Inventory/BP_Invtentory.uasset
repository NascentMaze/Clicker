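; Inventory Blueprint that stores items as class-and-amount slots, in an array sized to AmountOfSlots on BeginPlay.
; AddItem tops up partial stacks of stackable items, then uses empty slots found by linear search; non-stackable items take one slot each.
; Overflow recurses into AddItem, but the recursive result is ignored, so partial adds still return true.
; Query functions report slot emptiness and read item info from class defaults.
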(event `self.ReceiveBeginPlay`
  (`KismetArrayLibrary.Array_Resize` (`self.Slots`) (`self.AmountOfSlots`)))

(fn `AddItem`
  (params (ItemClass :type "/Game/Blueprints/Items/Classes/Item_Base Class Reference") (Amount :type Integer))
  (returns (`Succes?` :type Boolean))
  (locals (LocalClass :type "/Game/Blueprints/Items/Classes/Item_Base Class Reference") (LocalAmount :type Integer) (FoundIndex :type Integer))
  (bind _returnvalue (+ (`.Amount_5_BCDF298D42310F87AEE23DAD8A8111EC` (break `/Game/Blueprints/Items/Inventory/S_InventorySlot` (`|GetArrayItem` (`self.Slots`) (`local.FoundIndex`)))) (`local.LocalAmount`)))
  (set `local.LocalClass` ItemClass)
  (set `local.LocalAmount` Amount)
  (if (`.IsStackable?_15_3B3990B6491A501FDD5BB4911BB97653` (break `/Game/Blueprints/Items/S_ItemInfo` (defaults `/Game/Blueprints/Items/Inventory/BP_Invtentory` ItemClass)))
    (bind (_succes_ _index) (`self.SearchFreeStack` (`local.LocalClass`)))
    (if _succes_
      (set `local.FoundIndex` _index)
      (if (> _returnvalue (`self.MaxStackSize`))
        (set `local.LocalAmount` (- _returnvalue (`self.MaxStackSize`)))
        (`KismetArrayLibrary.Array_Set` (`self.Slots`) (`local.FoundIndex`) (make `/Game/Blueprints/Items/Inventory/S_InventorySlot` (`local.LocalClass`) (`self.MaxStackSize`)))
        (`self.AddItem` (`local.LocalClass`) (`local.LocalAmount`))
        (return true)
        (else
          (`KismetArrayLibrary.Array_Set` (`self.Slots`) (`local.FoundIndex`) (make `/Game/Blueprints/Items/Inventory/S_InventorySlot` (`local.LocalClass`) _returnvalue))
          (return true)))
      (else
        (bind (_success _index_2) (`self.SearchEmptySlot`))
        (if _success
          (bind _output_get (set `local.FoundIndex` _index_2))
          (if (> (`local.LocalAmount`) (`self.MaxStackSize`))
            (`KismetArrayLibrary.Array_Set` (`self.Slots`) _output_get (make `/Game/Blueprints/Items/Inventory/S_InventorySlot` (`local.LocalClass`) (`self.MaxStackSize`)))
            (`self.AddItem` (`local.LocalClass`) (- (`local.LocalAmount`) (`self.MaxStackSize`)))
            (return true)
            (else
              (`KismetArrayLibrary.Array_Set` (`self.Slots`) (`local.FoundIndex`) (make `/Game/Blueprints/Items/Inventory/S_InventorySlot` (`local.LocalClass`) (`local.LocalAmount`)))
              (return true)))
          (else
            (return false)))))
    (else
      (bind (_success_2 _index_3) (`self.SearchEmptySlot`))
      (if _success_2
        (bind _output_get_2 (set `local.FoundIndex` _index_3))
        (`KismetArrayLibrary.Array_Set` (`self.Slots`) _output_get_2 (make `/Game/Blueprints/Items/Inventory/S_InventorySlot` (`local.LocalClass`) 1))
        (if (> (`local.LocalAmount`) 1)
          (`self.AddItem` (`local.LocalClass`) (- (`local.LocalAmount`) 1))
          (return true)
          (else
            (return true)))
        (else
          (return false))))))

(fn `GetItemInfoAtIndex`
  (params (Index :type Integer))
  (returns (`EmptySlot?` :type Boolean) (ItemInfo :type "/Game/Blueprints/Items/S_ItemInfo Structure") (Amount :type Integer))
  (bind (_itemclass _amount) (break `/Game/Blueprints/Items/Inventory/S_InventorySlot` (`|GetArrayItem` (`self.Slots`) Index)))
  (if (`KismetSystemLibrary.IsValidClass` _itemclass)
    (return false (defaults `/Game/Blueprints/Items/Inventory/BP_Invtentory` _itemclass) _amount)
    (else
      (return false (struct) 0))))

(fn `IsSlotEmpty?`
  (params (Index :type Integer))
  (returns (`Empty?` :type Boolean))
  (return (not (`KismetSystemLibrary.IsValidClass` (`.ItemClass_2_F06F3F3E412E87AA5001A9ADE20BD893` (break `/Game/Blueprints/Items/Inventory/S_InventorySlot` (`|GetArrayItem` (`self.Slots`) Index)))))))

(fn `SearchEmptySlot`
  (returns (Success :type Boolean) (Index :type Integer))
  (locals (LocalBool :type Boolean) (LocalIndex :type Integer))
  (for (_array_element _array_index) (`self.Slots`)
    (if (not (`KismetSystemLibrary.IsValidClass` (`.ItemClass_2_F06F3F3E412E87AA5001A9ADE20BD893` (break `/Game/Blueprints/Items/Inventory/S_InventorySlot` _array_element))))
      (set `local.LocalBool` false)
      (set `local.LocalIndex` _array_index)
      (break)))
  (return (`local.LocalBool`) (`local.LocalIndex`)))

(fn `SearchFreeStack`
  (params (`Item Class` :type "/Game/Blueprints/Items/Classes/Item_Base Class Reference"))
  (returns (`Succes?` :type Boolean) (Index :type Integer))
  (locals (LocalBool :type Boolean) (LocalIndex :type Integer))
  (for (_array_element _array_index) (`self.Slots`)
    (bind (_itemclass _amount) (break `/Game/Blueprints/Items/Inventory/S_InventorySlot` _array_element))
    (if (`KismetSystemLibrary.IsValidClass` _itemclass)
      (if (and (== _itemclass `Item Class`) (< _amount (`self.MaxStackSize`)))
        (set `local.LocalBool` true)
        (set `local.LocalIndex` _array_index)
        (break))))
  (return (`local.LocalBool`) (`local.LocalIndex`)))

(fn `UserConstructionScript`)